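; Wave manager that spawns endless waves of BP_EnemigoBase, each larger and with a spawn interval that shortens down to a clamp.
; IniciarOleada sets the counters and, if the player HUD is valid, updates it and starts the looping SpawnearUnEnemigo timer.
; Each spawn uses random spawn points and calls AumentarEstadisticasDelEnemigo on all enemies of ClaseDeEnemigo's class, not just the new one.
; RestarEnemigoRestante decrements the HUD-mirrored count; the timer advances waves once both counters empty.
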(event `Estadisticas`
  (bind _returnvalue (`|GetDataTableRow` (`self.Table`) (`KismetStringLibrary.Conv_StringToName` (`KismetStringLibrary.Conv_IntToString` (`self.OleadaActual`))))))

(event `self.ReceiveBeginPlay`
  (set `self.OleadaActual` 1)
  (`self.IniciarOleada`)
  (bind _asbp_enemigo_base (cast `/Game/DeDani/BluePrints/BP_EnemigoBase` (`self.ClaseDeEnemigo`)))
  (set `self.ClaseDeEnemigo` _asbp_enemigo_base))

(event `IniciarOleada`
  (bind _output_get (set `self.CantidadDeEnemigosPorOleada` (* (`self.OleadaActual`) 3)))
  (bind _output_get_2 (set `self.EnemigosRestantes` _output_get))
  (set `self.EnemigosPorSpawnear` _output_get_2)
  (`KismetSystemLibrary.Delay` 0.2)
  (bind _outactors (`GameplayStatics.GetAllActorsOfClass` "/Game/TopDown/Blueprints/BP_Jugador.BP_Jugador_C"))
  (bind _w_hudjugadorref (`/Game/TopDown/Blueprints/BP_Jugador.W_HUDJugadorRef` (`|GetArrayItem` _outactors)))
  (`/Engine/EditorBlueprintResources/StandardMacros.IsValid` _w_hudjugadorref
    (:`Is Valid`
      (set `/Game/DeDani/Widget/W_HUDJugador.OleadaActual` (`self.OleadaActual`) _w_hudjugadorref)
      (set `/Game/DeDani/Widget/W_HUDJugador.EnemigosRestantes` (`self.EnemigosRestantes`) _w_hudjugadorref)
      (bind _output_get_3 (set `self.TiempoDeSpawn` (`KismetMathLibrary.FClamp` (- (`self.TiempoEntreSpawns`) (* (`self.OleadaActual`) (`self.ReduccionPorOleada`))))))
      (`KismetSystemLibrary.K2_SetTimer` null "SpawnearUnEnemigo" _output_get_3 true))
    (:`Is Not Valid`
      (`KismetSystemLibrary.PrintString` "No Es Valido Oleadas"))))

(fn `RestarEnemigoRestante`
  (set `self.EnemigosRestantes` (- (`self.EnemigosRestantes`) 1))
  (bind _outactors (`GameplayStatics.GetAllActorsOfClass` "/Game/TopDown/Blueprints/BP_Jugador.BP_Jugador_C"))
  (bind _w_hudjugadorref (`/Game/TopDown/Blueprints/BP_Jugador.W_HUDJugadorRef` (`|GetArrayItem` _outactors)))
  (`/Engine/EditorBlueprintResources/StandardMacros.IsValid` _w_hudjugadorref
    (:`Is Valid`
      (set `/Game/DeDani/Widget/W_HUDJugador.EnemigosRestantes` (`self.EnemigosRestantes`) _w_hudjugadorref))
    (:`Is Not Valid`
      (`KismetSystemLibrary.PrintString` "No es validoEnemigo"))))

(fn `SpawnearUnEnemigo`
  (bind _outitem (`KismetArrayLibrary.Array_Random` (`self.PuntosDeSpawn`)))
  (if (and (<= (`self.EnemigosPorSpawnear`) 0) (<= (`self.EnemigosRestantes`) 0))
    (set `self.OleadaActual` (+ (`self.OleadaActual`) 1))
    (`KismetSystemLibrary.K2_ClearTimer` null "SpawnearUnEnemigo")
    (`self.IniciarOleada`)
    (elif (> (`self.EnemigosPorSpawnear`) 0)
      (`|SpawnActorFromClass` "/Game/DeDani/BluePrints/BP_EnemigoBase.BP_EnemigoBase_C" (`KismetMathLibrary.MakeTransform` (`self.K2_GetActorLocation` _outitem) (`self.K2_GetActorRotation` _outitem)) "Undefined" "MultiplyWithRoot" null null)
      (set `self.EnemigosPorSpawnear` (- (`self.EnemigosPorSpawnear`) 1))
      (bind _outactors (`GameplayStatics.GetAllActorsOfClass` (`GameplayStatics.GetObjectClass` (`self.ClaseDeEnemigo`))))
      (for _array_element _outactors
        (`/Game/DeDani/BluePrints/BP_EnemigoBase.AumentarEstadisticasDelEnemigo` _array_element)))))

(fn `UserConstructionScript`)