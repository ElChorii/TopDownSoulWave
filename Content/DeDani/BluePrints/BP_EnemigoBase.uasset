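; Base enemy pawn for a wave-based game that chases the player through AI MoveTo, reissued every tick.
; Capsule overlap calls the player's damage function, then writes this enemy's Daño to the player afterwards.
; RecibirDañoEnemigo subtracts the player's DañoBase; at zero health it grants XP, decrements BP_GestorOleadas' remaining count and destroys itself.
; AumentarEstadisticasDelEnemigo scales max health, damage and XP by wave, leaving current health untouched.
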(event `self.ReceiveTick`
  (params (DeltaSeconds :type "Float (single-precision)"))
  (cast `AIController` (`self.GetController`))
  (`|AIMoveTo` self (0.0 0.0 0.0) (`GameplayStatics.GetPlayerPawn` 0) 1.0))

(event `self.CapsuleComponent.OnComponentBeginOverlap`
  (params (OverlappedComponent :type "PrimitiveComponent Object Reference") (OtherActor :type "Actor Object Reference") (OtherComp :type "PrimitiveComponent Object Reference") (OtherBodyIndex :type Integer) (bFromSweep :type Boolean) (SweepResult :type "HitResult Structure (by ref)"))
  (bind _asbp_jugador (cast `/Game/TopDown/Blueprints/BP_Jugador` OtherActor))
  (`/Game/TopDown/Blueprints/BP_Jugador.RecibirDañoJugador` _asbp_jugador)
  (set `/Game/TopDown/Blueprints/BP_Jugador.Cantidad de daño Recibido Del Enemigo` (`self.Daño`) _asbp_jugador))

(fn `AumentarEstadisticasDelEnemigo`
  (bind _vidamaxima (`self.VidaMaxima`))
  (bind `_daño` (`self.Daño`))
  (bind _experienciaquedaelenemigo (`self.ExperienciaQueDaElEnemigo`))
  (set `self.VidaMaxima` (+ _vidamaxima (* _vidamaxima (* (`self.Oleada Actual`) (`self.AumentoPorOleada`)))))
  (set `self.Daño` (+ `_daño` (* `_daño` (* (`self.Oleada Actual`) (`self.AumentoPorOleada`)))))
  (set `self.ExperienciaQueDaElEnemigo` (+ _experienciaquedaelenemigo (* _experienciaquedaelenemigo (* (`self.Oleada Actual`) (`self.AumentoPorOleada`))))))

(fn `RecibirDañoEnemigo`
  (bind _asbp_jugador (cast `/Game/TopDown/Blueprints/BP_Jugador` (`GameplayStatics.GetPlayerPawn` 0)))
  (set `self.VidaActual` (- (`self.VidaActual`) (`/Game/TopDown/Blueprints/BP_Jugador.DañoBase` _asbp_jugador)))
  (if (<= (`self.VidaActual`) 0.0)
    (set `/Game/TopDown/Blueprints/BP_Jugador.ExperienciaRecibida` (`self.ExperienciaQueDaElEnemigo`) _asbp_jugador)
    (`/Game/TopDown/Blueprints/BP_Jugador.RecibirExp` _asbp_jugador)
    (bind _outactors (`GameplayStatics.GetAllActorsOfClass` "/Game/DeDani/BluePrints/BP_GestorOleadas.BP_GestorOleadas_C"))
    (`/Game/DeDani/BluePrints/BP_GestorOleadas.RestarEnemigoRestante` (`|GetArrayItem` _outactors))
    (`self.K2_DestroyActor`)))

(fn `UserConstructionScript`)